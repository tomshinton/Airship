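; Bullet ammo actor that moves as a physics-simulated mesh and leaves a debug trail of its path.
; On BeginPlay it flushes persistent debug lines, enables physics on ItemMesh and starts a looping timer.
; Each timer tick draws a timed green line from the last recorded mesh position to the current one.
; Flushing on every spawn also wipes trails left by earlier bullets.
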(event Custom|DrawTrail
  (bind _itemmesh (Variables|Default|GetItemMesh))
  (bind _returnvalue (Transformation|GetWorldLocation _itemmesh))
  (Rendering|Debug|DrawDebugLine (Variables|Default|GetLastPosition) _returnvalue "(R=0.047154,G=0.515625,B=0.000000,A=1.000000)" 15.0 2.0)
  (Variables|Default|SetLastPosition _returnvalue))

(event EventBeginPlay
  (Rendering|Debug|FlushPersistentDebugLines)
  (Physics|SetSimulatePhysics (Variables|Default|GetItemMesh) true)
  (Variables|Default|SetLastPosition (Transformation|GetWorldLocation (Variables|Default|GetItemMesh)))
  (Utilities|Time|SetTimerbyEvent (delegate Custom|DrawTrail) 0.2 true))

(fn ConstructionScript)
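; ItemProvider is a world actor that stocks a resource in its AirInventory and hands one unit to the player's inventory on each interaction.
; It seeds five units at BeginPlay, and a text label shows resource, stack count and total, set at construction and after each transfer.
; The label yaws toward the player every tick.
; A Refresh event adds one unit, but its looping timer is never run.
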(event Custom|Refresh
  (Class|AirInventory|AddItem (Variables|Default|GetAirInventory) (Variables|Default|GetResource) 1)
  (CallFunction|UpdateReadout))

(event Custom|UpdateReadout
  (bind _resource (Variables|Default|GetResource))
  (bind (_stacks _total) (Class|AirInventory|Audit (Variables|Default|GetAirInventory) _resource))
  (Rendering|Components|TextRender|SetText (Variables|Default|GetTextRender) (Utilities|Text|ToText(String) (Utilities|String|Append (Utilities|String|ToString(Name) _resource) " x " (Utilities|String|ToString(Integer) _stacks) " (" (Utilities|String|ToString(Integer) _total) ")"))))

(event Collision|EventActorBeginOverlap
  (params (OtherActor :type Actor%20Object%20Reference)))

(event EventTick
  (params (DeltaSeconds :type Float%20%28single-precision%29))
  (Transformation|SetWorldRotation (Variables|Default|GetTextRender) (Math|Rotator|MakeRotator 0.0 0.0 (.yaw (Math|Rotator|FindLookatRotation (Transformation|GetActorLocation) (Transformation|GetActorLocation (Game|GetPlayerCharacter 0))))) false false))

(event EventOnInteract
  (bind _asair_char (Utilities|Casting|CastToAirChar (Game|GetPlayerCharacter 0)))
  (Class|AirInventory|TransferItem (Class|AirChar|GetInventory _asair_char) (Variables|Default|GetResource) 1 (Variables|Default|GetAirInventory))
  (CallFunction|UpdateReadout))

(event EventBeginPlay
  (Class|AirInventory|AddItem (Variables|Default|GetAirInventory) (Variables|Default|GetResource) 5))

(fn ConstructionScript
  (bind _resource (Variables|Default|GetResource))
  (bind (_stacks _total) (Class|AirInventory|Audit (Variables|Default|GetAirInventory) _resource))
  (Rendering|Components|TextRender|SetText (Variables|Default|GetTextRender) (Utilities|Text|ToText(String) (Utilities|String|Append (Utilities|String|ToString(Name) _resource) " x " (Utilities|String|ToString(Integer) _stacks) " (" (Utilities|String|ToString(Integer) _total) ")"))))
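; Container is an interactable storage actor that moves its configured Resource types between its AirInventory and the player's AirChar inventory.
; Each interaction alternates via FlipFlop, first depositing from the player, then withdrawing to the player, requesting a fixed quantity of each resource.
; The construction script concatenates resource names into a TextRender label, which yaws every tick to face the player.
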(event Collision|EventActorBeginOverlap
  (params (OtherActor :type Actor%20Object%20Reference)))

(event EventTick
  (params (DeltaSeconds :type Float%20%28single-precision%29))
  (Transformation|SetWorldRotation (Variables|Default|GetTextRender) (Math|Rotator|MakeRotator 0.0 0.0 (.yaw (Math|Rotator|FindLookatRotation (Transformation|GetActorLocation) (Transformation|GetActorLocation (Game|GetPlayerCharacter 0))))) false false))

(event EventOnInteract
  (Utilities|FlowControl|FlipFlop
    (:A
      (bind _asair_char (Utilities|Casting|CastToAirChar (Game|GetPlayerCharacter 0)))
      (for _array_element (Variables|Default|GetResource)
        (Class|AirInventory|TransferItem (Variables|Default|GetAirInventory) _array_element 100 (Class|AirChar|GetInventory _asair_char))))
    (:B
      (bind _asair_char_2 (Utilities|Casting|CastToAirChar (Game|GetPlayerCharacter 0)))
      (for _array_element_2 (Variables|Default|GetResource)
        (Class|AirInventory|TransferItem (Class|AirChar|GetInventory _asair_char_2) _array_element_2 100 (Variables|Default|GetAirInventory))))))

(event EventBeginPlay)

(fn ConstructionScript
  (for _array_element (Variables|Default|GetResource)
    (bind _output_get (Variables|Default|SetReadout (Utilities|String|Append (Variables|Default|GetReadout) " 
" (Utilities|String|ToString(Name) _array_element))))
    (Rendering|Components|TextRender|SetText (Variables|Default|GetTextRender) (Utilities|Text|ToText(String) _output_get))))